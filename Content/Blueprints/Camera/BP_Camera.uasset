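; BP_Camera is a follow camera that trails a target actor at the offset captured when the target is set.
; Each tick it eases toward that position and rotates toward the target's eye height.
; When line traces find the view blocked, it steps along a line toward a fallback point directly above the target, taking the first clear spot.
; TryBlockedView is an empty hook receiving the traced hit actor.
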(event `self.ReceiveBeginPlay`
  (`self.ChangeTargetActor` (`self.Target`)))

(event `self.ReceiveTick`
  (params (DeltaSeconds :type "Float (single-precision)"))
  (`self.UpdatePosition`)
  (`self.UpdateRotation`))

(fn `CanSeeTargetFrom`
  (params (Position :type "Vector Structure"))
  (returns (IsVisible :type Boolean))
  (bind (_outhit _returnvalue) (`KismetSystemLibrary.LineTraceSingle` Position (`self.GetlookAtPosition`) "TraceTypeQuery1" false (`|MakeArray` (`self.Target`))))
  (`self.TryBlockedView` (`.HitActor` (`GameplayStatics.BreakHitResult` _outhit)))
  (return (not _returnvalue)))

(fn `ChangeTargetActor`
  (params (NewTarget :type "Actor Object Reference"))
  (bind _returnvalue (- (`self.K2_GetActorLocation`) (`self.GetlookAtPosition`)))
  (bind _output_get (set `self.Target` NewTarget))
  (`/Engine/EditorBlueprintResources/StandardMacros.IsValid` _output_get
    (:`Is Valid`
      (set `self.TargetOffset` _returnvalue)
      (set `self.TargetDistance` (`KismetMathLibrary.VSize` _returnvalue)))))

(fn `GetlookAtPosition`
  (returns (Position :type "Vector Structure"))
  (return (+ (`self.K2_GetActorLocation` (`self.Target`)) (`KismetMathLibrary.MakeVector` 0.0 0.0 (`self.TargetEyesHeight`)))))

(fn `TryBlockedView`
  (params (Target :type "Actor Object Reference")))

(fn `UpdatePosition`
  (locals (SelectedPosition :type "Vector Structure"))
  (`/Engine/EditorBlueprintResources/StandardMacros.IsValid` (`self.Target`)
    (:`Is Valid`
      (set `local.SelectedPosition` (`self.GetNaturalPosition`))
      ;[1 1 1] Desired position
      (for _index (range 11)
        (bind _returnvalue (`KismetMathLibrary.VLerp` (`self.GetNaturalPosition`) (`self.GetLastResourcePosition`) (`KismetMathLibrary.NormalizeToRange` (`KismetMathLibrary.Conv_IntToDouble` _index) 0.0 10.0)))
        (bind _isvisible (`self.CanSeeTargetFrom` _returnvalue))
        (if _isvisible
          (set `local.SelectedPosition` _returnvalue)
          (break)))
      (`self.K2_SetActorLocation` (`KismetMathLibrary.VLerp` (`self.K2_GetActorLocation`) (`local.SelectedPosition`) (* (`self.TranslationSpeed`) (`GameplayStatics.GetWorldDeltaSeconds`)))))))

(fn `UpdateRotation`
  (`/Engine/EditorBlueprintResources/StandardMacros.IsValid` (`self.Target`)
    (:`Is Valid`
      (`self.K2_SetActorRotation` (`KismetMathLibrary.RLerp` (`self.K2_GetActorRotation`) (`KismetMathLibrary.FindLookAtRotation` (`self.K2_GetActorLocation`) (`self.GetlookAtPosition`)) (* (`self.RotationSpeed`) (`GameplayStatics.GetWorldDeltaSeconds`)))))))

(fn `UserConstructionScript`)