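; BP_CameraGhosting hides static meshes that sit between the third-person player character and its follow camera.
; Each tick it re-shows every stored mesh, then, while the character is the view target, multi-line traces from character to camera.
; Non-pawn hits have their static mesh components switched invisible rather than faded, and printed by name.
; Hidden components are appended to TransparentActors, which is never cleared.
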(event `self.ReceiveBeginPlay`
  (bind _output_get (set `self.PlayerCharacter` (`GameplayStatics.GetPlayerCharacter` 0)))
  (bind _asbp_third_person_character (cast `/Game/Blueprints/Player/BP_ThirdPersonCharacter` _output_get))
  (set `self.CameraRef` (`/Game/Blueprints/Player/BP_ThirdPersonCharacter.FollowCamera` _asbp_third_person_character)))

(event `self.ReceiveTick`
  (params (DeltaSeconds :type "Float (single-precision)"))
  (bind _cameraref (`self.CameraRef`))
  (bind _playercharacter (`self.PlayerCharacter`))
  (for _array_element (`self.TransparentActors`)
    (`SceneComponent.SetVisibility` _array_element true false))
  (if (== (`Controller.GetViewTarget` (`GameplayStatics.GetPlayerController` 0)) (`self.PlayerCharacter`))
    (if (`KismetSystemLibrary.IsValid` _cameraref)
      (bind (_outhits _returnvalue) (`KismetSystemLibrary.LineTraceMultiForObjects` (`Actor.K2_GetActorLocation` _playercharacter) (`SceneComponent.K2_GetComponentLocation` _cameraref) (`|MakeArray` "ObjectTypeQuery4" "ObjectTypeQuery1" "ObjectTypeQuery2" :!type "EObjectTypeQuery Enum") false (`|MakeArray` _playercharacter :!type "Actor Object Reference")))
      (if _returnvalue
        (for _array_element_2 _outhits
          (cast `Pawn` (`.HitActor` (`GameplayStatics.BreakHitResult` _array_element_2))
            (:`CastFailed`
              (`KismetSystemLibrary.PrintString` (`KismetSystemLibrary.GetDisplayName` (`.HitActor` (`GameplayStatics.BreakHitResult` _array_element_2))))
              (for _array_element_3 (`Actor.K2_GetComponentsByClass` (`.HitActor` (`GameplayStatics.BreakHitResult` _array_element_2)) "/Script/Engine.StaticMeshComponent")
                (`KismetArrayLibrary.Array_Add` (`self.TransparentActors`) _array_element_3)
                (`SceneComponent.SetVisibility` _array_element_3 false false)))))))))