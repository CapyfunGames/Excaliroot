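; BP_Radish is an explosive weapon actor, apparently a projectile, that detonates when it hits something.
; On Hit, Explode destroys the Sphere component, turns off physics on SphereCollision and uses that component's overlaps as the blast area.
; Overlapping BP_Enemy actors take damage, while other actors with physics-simulating roots get a constant-falloff radial impulse.
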(event `self.ReceiveActorBeginOverlap`
  (params (OtherActor :type "Actor Object Reference")))

(event `self.ReceiveHit`
  (params (MyComp :type "PrimitiveComponent Object Reference") (Other :type "Actor Object Reference") (OtherComp :type "PrimitiveComponent Object Reference") (bSelfMoved :type Boolean) (HitLocation :type "Vector Structure") (HitNormal :type "Vector Structure") (NormalImpulse :type "Vector Structure") (Hit :type "HitResult Structure (by ref)"))
  (`self.Explode`))

(fn `Explode`
  (`ActorComponent.K2_DestroyComponent` (`self.Sphere`))
  (`PrimitiveComponent.SetSimulatePhysics` (`self.Sphere Collision`) false)
  (for _array_element (`PrimitiveComponent.GetOverlappingActors` (`self.Sphere Collision`) null)
    (bind _asbp_enemy (cast `/Game/Blueprints/Enemies/BP_Enemy` _array_element)
      (:`then`
        (`GameplayStatics.ApplyDamage` _asbp_enemy (`self.Damage`) null self))
      (:`CastFailed`
        (bind _rootcomponent (`Actor.RootComponent` _array_element))
        (if (`SceneComponent.IsSimulatingPhysics` _rootcomponent "None")
          (`PrimitiveComponent.AddRadialImpulse` (cast `PrimitiveComponent` _rootcomponent :!pure true) (`self.K2_GetActorLocation`) (`SphereComponent.SphereRadius` (`self.Sphere Collision`)) 4000.0 "RIF_Constant" true))))))

(fn `UserConstructionScript`
  (`parent.UserConstructionScript`))