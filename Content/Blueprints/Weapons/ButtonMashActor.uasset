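; Weapon pickup actor that makes the player button-mash to pull a spawned weapon out.
; TryPick shows the mash widget and retargets porcupine enemies on first press, then each press shakes the camera and decrements a count set only at BeginPlay.
; At zero, Pick attaches the weapon to the character's socket, plays dirt effects, disables collision, triggers respawn and sends porcupines to "Wall".
; The spawner's spawned-weapon event re-enables collision.
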(event `self.ReceiveBeginPlay`
  (set `self.CurrentCount` (`self.ButtonMashCount`))
  (bind _returnvalue (`NiagaraFunctionLibrary.SpawnSystemAtLocation` "/Game/Particles/P_Poof.P_Poof" (`SceneComponent.K2_GetComponentLocation` (`self.DefaultSceneRoot`)) (struct) (1.0 1.0 1.0) false false))
  (set `self.ParticleSystem` _returnvalue)
  (add `/Game/Blueprints/Spawner/BP_Spawner.SpawnedWeapon` (`self.WeaponSpawner`) (delegate `ResetCollisions`)))

(event `ResetCollisions`
  (`self.SetActorEnableCollision` true)
  (set `PrimitiveComponent.bGenerateOverlapEvents` true (`self.Sphere`)))

(event `SpawnParticles`
  (bind _particlesystem (`self.ParticleSystem`))
  (`ActorComponent.Activate` _particlesystem false)
  (`KismetSystemLibrary.Delay` 2.0)
  (`ActorComponent.Deactivate` _particlesystem))

(fn `Pick`
  (params (ParentActor :type "Actor Object Reference"))
  (returns (OutWeapon :type "Actor Object Reference"))
  (bind _weaponspawner (`self.WeaponSpawner`))
  (bind _spawnedactor (`/Game/Blueprints/Spawner/BP_Spawner.spawnedActor` _weaponspawner))
  (bind _asbp_third_person_character (cast `/Game/Blueprints/Player/BP_ThirdPersonCharacter` ParentActor))
  (`self.K2_AttachToComponent` _spawnedactor (`Character.Mesh` _asbp_third_person_character) "weapon_socket" "SnapToTarget" "KeepRelative" "KeepRelative" true)
  (`self.SetActorEnableCollision` false)
  (set `PrimitiveComponent.bGenerateOverlapEvents` false (`self.Sphere`))
  (`GameplayStatics.PlaySound2D` "/Game/Sound/Dirt.Dirt" 1.0 1.0 0.0 null null)
  (`self.SpawnParticles`)
  (bind _asbp_roots_spawner (cast `/Game/Blueprints/Spawner/BP_RootsSpawner` _weaponspawner))
  (`/Game/Blueprints/Spawner/BP_RootsSpawner.RespawnWeapon` _asbp_roots_spawner)
  (set `self.Picking` false)
  (bind _asexcalli_root_game_mode (cast `/Game/Blueprints/ExcalliRootGameMode` (`GameplayStatics.GetGameMode`)))
  (`/Game/Blueprints/ExcalliRootGameMode.ChangeEnemyObjective` _asexcalli_root_game_mode "" "Wall" "/Game/Blueprints/Enemies/BP_Porcupine.BP_Porcupine_C")
  (return _spawnedactor))

(fn `TryPick`
  (params (ParentActor :type "Actor Object Reference"))
  (returns (OutWeapon :type "Actor Object Reference"))
  (if (not (`self.Picking`))
    (bind _returnvalue (`|CreateWidget` "/Game/Blueprints/UI/WBP_ButtonMash.WBP_ButtonMash_C"))
    (set `self.Widget` _returnvalue)
    (`UserWidget.AddToViewport` _returnvalue 0)
    (set `self.Picking` true)
    (bind _asexcalli_root_game_mode (cast `/Game/Blueprints/ExcalliRootGameMode` (`GameplayStatics.GetGameMode`)))
    (`/Game/Blueprints/ExcalliRootGameMode.ChangeEnemyObjective` _asexcalli_root_game_mode "" "/Game/Blueprints/Enemies/BP_Porcupine.BP_Porcupine_C"))
  (bind _output_get (set `self.CurrentCount` (- (`self.CurrentCount`) 1)))
  (`GameplayStatics.PlayWorldCameraShake` "/Game/Blueprints/Camera/BP_EpicShake.BP_EpicShake_C" (`self.K2_GetActorLocation`) 0.0 5000.0)
  (if (<= _output_get 0)
    (`Widget.RemoveFromParent` (`self.Widget`))
    (bind _outweapon (`self.Pick` (`local.ParentActor`)))
    (return _outweapon)))

(fn `UserConstructionScript`)