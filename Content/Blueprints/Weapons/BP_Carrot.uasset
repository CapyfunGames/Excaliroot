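; BP_Carrot is a carrot weapon Blueprint that wears out after a limited number of hits.
; On BeginPlay it sets its Type enum, then runs the parent's BeginPlay.
; Every actor overlap calls Attack, with no filter on the other actor.
; Attack only decrements HitsLeft and destroys the carrot when the count reaches exactly zero, applying no damage itself.
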(event `self.ReceiveBeginPlay`
  ;[1 1 1] Set start variables
  (set `self.Type` "NewEnumerator1")
  (`parent.ReceiveBeginPlay`))

(event `self.ReceiveActorBeginOverlap`
  (params (OtherActor :type "Actor Object Reference"))
  ;[1 1 1] Attack when overlap
  (`self.Attack`))

(fn `Attack`
  (bind _output_get (set `self.HitsLeft` (- (`self.HitsLeft`) 1)))
  (if (== _output_get 0)
    (`self.K2_DestroyActor`)))

(fn `UserConstructionScript`
  (`parent.UserConstructionScript`))