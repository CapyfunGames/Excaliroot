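; BP_RootsSpawner is a spawner child Blueprint that calls Spawn with its configured weapon type and a fixed enemy type, once at BeginPlay.
; RespawnWeapon repeats that Spawn call after a short delay.
; Each spawn triggers a P_Poof particle burst from a system created once at the spawner's location, activated and then deactivated after a delay rather than destroyed.
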(event `self.ReceiveBeginPlay`
  (bind _returnvalue (`NiagaraFunctionLibrary.SpawnSystemAtLocation` "/Game/Particles/P_Poof.P_Poof" (`self.K2_GetActorLocation` self) (struct) (1.0 1.0 1.0) false false))
  (set `self.PoofSystem` _returnvalue)
  (`self.Spawn` (`self.TypeOfWeapon`))
  (`self.SpawningParticles` :!label _label))

(event `RespawnWeapon`
  (`KismetSystemLibrary.Delay` 2.0)
  (`self.Spawn` (`self.TypeOfWeapon`))
  (goto _label))

(event `SpawningParticles`
  (bind _poofsystem (`self.PoofSystem`))
  (`ActorComponent.Activate` _poofsystem false)
  (`KismetSystemLibrary.Delay` 2.0)
  (`ActorComponent.Deactivate` _poofsystem))

(fn `UserConstructionScript`
  (`parent.UserConstructionScript`))