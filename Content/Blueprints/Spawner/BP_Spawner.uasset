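; BP_Spawner is a spawner actor that places a carrot weapon or an enemy at its Box, depending on SpawnedType.
; Spawn stores the SpawnWeapon result, a scaled, offset BP_Carrot, as SpawnedActor; the Enemy branch has no class set.
; BeginPlay and end-overlap events are empty.
; Disconnected EventGraph logic would spawn a carrot, including a delayed respawn for the tracked actor, but never runs.
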(event `self.ReceiveBeginPlay`)

(event `self.Box.OnComponentEndOverlap`
  (params (OverlappedComponent :type "PrimitiveComponent Object Reference") (OtherActor :type "Actor Object Reference") (OtherComp :type "PrimitiveComponent Object Reference") (OtherBodyIndex :type Integer)))

(fn `Spawn`
  (params (WeaponType :type "/Game/Blueprints/Data/E_WeaponTypes Enum" :default "NewEnumerator1"))
  (bind _returnvalue (`SceneComponent.K2_GetComponentLocation` (`self.Box`)))
  (switch `/Game/Blueprints/Data/EBP_SpawnedType` (`self.spawnedType`)
    (:`NewEnumerator0`
      (bind _spawnedweapon (`self.SpawnWeapon` (`local.WeaponType`) (`KismetMathLibrary.MakeTransform` (+ (`self.SpawnOffset`) _returnvalue) (struct) (`self.SpawnScale`)))))
    (:`NewEnumerator1`
      (`|SpawnActorFromClass` "/Game/Blueprints/Spawner/BP_SpawneableActor.BP_SpawneableActor_C" (`KismetMathLibrary.Conv_VectorToTransform` _returnvalue) "Undefined" "OverrideRootScale" null null)))
  (set `self.spawnedActor` _spawnedweapon))

(fn `SpawnWeapon`
  (params (WeaponType :type "/Game/Blueprints/Data/E_WeaponTypes Enum" :default "NewEnumerator1") (SpawnTransform :type "Transform Structure"))
  (returns (SpawnedWeapon :type "Actor Object Reference"))
  (switch `/Game/Blueprints/Data/E_WeaponTypes` WeaponType
    (:`NewEnumerator1`
      (bind _returnvalue (`|SpawnActorFromClass` "/Game/Blueprints/Weapons/BP_Carrot.BP_Carrot_C" SpawnTransform "Undefined" "OverrideRootScale" null null))
      (return _returnvalue))))

(fn `UserConstructionScript`)