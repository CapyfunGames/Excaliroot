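; BP_Wall is a damageable wall actor whose destruction ends the game.
; It sets its remaining health to the maximum on BeginPlay and subtracts the amount of any damage it receives.
; When health reaches zero or below, it casts the game mode to ExcalliRootGameMode and calls ShowGameOver.
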(event `self.ReceiveBeginPlay`
  (set `self.HealthLeft` (`self.MaxHealth`)))

(event `self.ReceiveAnyDamage`
  (params (Damage :type "Float (single-precision)") (DamageType :type "DamageType Object Reference") (InstigatedBy :type "Controller Object Reference") (DamageCauser :type "Actor Object Reference"))
  (bind _output_get (set `self.HealthLeft` (- (`self.HealthLeft`) Damage)))
  (if (<= _output_get 0.0)
    (bind _asexcalli_root_game_mode (cast `/Game/Blueprints/ExcalliRootGameMode` (`GameplayStatics.GetGameMode`)))
    (`/Game/Blueprints/ExcalliRootGameMode.Show GameOver` _asexcalli_root_game_mode)))

(fn `UserConstructionScript`)