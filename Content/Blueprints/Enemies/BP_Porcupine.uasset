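; BP_Porcupine is an enemy Blueprint that repeatedly damages its AttackTarget while attacking.
; Attack and StopAttack toggle IsAttacking, and StopAttack also zeroes the cooldown Timer.
; Tick counts Timer down and, when it expires during an attack, plays the Attackito timeline.
; Each timeline update applies Damage and resets Timer to MaxTimer, so one play can deal multiple hits.
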(event `self.ReceiveTick`
  (params (DeltaSeconds :type "Float (single-precision)"))
  (set `self.Timer` (- (`self.Timer`) DeltaSeconds))
  (if (and (`self.IsAttacking`) (<= (`self.Timer`) 0.0))
    (`Timeline|Attackito`
      (:`Update`
        (`GameplayStatics.ApplyDamage` (`self.AttackTarget`) (`self.Damage`))
        (set `self.Timer` (`self.MaxTimer`))))))

(fn `Attack`
  (set `self.IsAttacking` true))

(fn `Stop Attack`
  (set `self.Timer` 0.0)
  (set `self.IsAttacking` false))

(fn `UserConstructionScript`
  (`parent.UserConstructionScript`))