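; Game mode for ExcalliRoot that handles the game UI, play timer, game-over screen and enemy targeting.
; BeginPlay shows the HUD and resets the timer, which Tick advances about once per second through a Delay while IsGaming is set.
; ShowGameOver swaps in the game-over widget but sets IsGaming true, so timing continues.
; Other events retarget all BP_Enemy actors to the player and close the controller's options menu.
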(event `self.ReceiveBeginPlay`
  (bind _returnvalue (`|CreateWidget` "/Game/Blueprints/UI/WBP_GameUI.WBP_GameUI_C"))
  (`UserWidget.AddToViewport` _returnvalue 0)
  (`self.InitGame`))

(event `Show GameOver`
  (bind _returnvalue (`|CreateWidget` "/Game/Blueprints/UI/WBP_GameOver.WBP_GameOver_C"))
  (`UserWidget.AddToViewport` _returnvalue 0)
  (`Widget.RemoveFromParent` (stale `self.ReceiveBeginPlay` _returnvalue))
  (set `self.isGaming` true))

(event `self.ReceiveTick`
  (params (DeltaSeconds :type "Float (single-precision)"))
  (`KismetSystemLibrary.Delay` 1.0)
  (if (`self.isGaming`)
    (`self.IncreaseTime`)))

(event `ChangeEnemyObjective`
  (params (PlayerObjective :type String))
  (bind _outactors (`GameplayStatics.GetAllActorsOfClass` "/Game/Blueprints/Enemies/BP_Enemy.BP_Enemy_C"))
  (if (`KismetStringLibrary.EqualEqual_StrStr` PlayerObjective "Player")
    (set `self.EnemyObjective` (`GameplayStatics.GetPlayerPawn` 0))
    (for _array_element _outactors
      (set `/Game/Blueprints/Enemies/BP_Enemy.AttackTarget` (`self.EnemyObjective`) _array_element))))

(event `CloseOptionsMenu`
  (bind _asbp_player_controller (cast `/Game/Blueprints/Player/BP_PlayerController` (`GameplayStatics.GetPlayerController` 0)))
  (`/Game/Blueprints/Player/BP_PlayerController.CloseOptions` _asbp_player_controller))

(fn `IncreaseTime`
  (bind _result (`/Engine/EditorBlueprintResources/StandardMacros.IncrementInt` (`self.Seconds`))
    (:`  `
      (if (> _result 59)
        (`/Engine/EditorBlueprintResources/StandardMacros.IncrementInt` (`self.Minutes`)
          (:`  `
            (set `self.Seconds` 0)))))))

(fn `InitGame`
  (set `self.Seconds` 0)
  (set `self.Minutes` 0)
  (set `self.isGaming` true))

(fn `UserConstructionScript`)