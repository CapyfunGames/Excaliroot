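; Controller for the player's grab sequence, switching camera and movement while a button-mash pickup is in progress.
; It tracks the ButtonMashActor overlapping the player character through overlap events bound at BeginPlay.
; Every Tick, active picking blends the view to the character's PickingCamera and disables movement.
; Otherwise, Tick blends back to the character and reapplies the movement mode cached at BeginPlay.
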(event `self.ReceiveBeginPlay`
  (bind _asbp_third_person_character (cast `/Game/Blueprints/Player/BP_ThirdPersonCharacter` (`GameplayStatics.GetPlayerCharacter` 0)))
  (bind _output_get (set `self.PlayerCharacter` _asbp_third_person_character))
  (add `Actor.OnActorBeginOverlap` _output_get (delegate `OnBeginOverlap`))
  (add `Actor.OnActorEndOverlap` _output_get (delegate `OnEndOverlap`))
  (set `self.CameraManager` (`GameplayStatics.GetPlayerCameraManager` 0))
  (set `self.PlayerController` (`GameplayStatics.GetPlayerController` 0))
  (set `self.MovementMode` (`CharacterMovementComponent.MovementMode` (`Character.CharacterMovement` (`self.PlayerCharacter`)))))

(event `OnBeginOverlap`
  (params (OverlappedActor :type "Actor Object Reference") (OtherActor :type "Actor Object Reference"))
  (bind _asbutton_mash_actor (cast `/Game/Blueprints/Weapons/ButtonMashActor` OtherActor))
  (set `self.CurrentButtonMash` _asbutton_mash_actor))

(event `OnEndOverlap`
  (params (OverlappedActor :type "Actor Object Reference") (OtherActor :type "Actor Object Reference"))
  (cast `/Game/Blueprints/Weapons/ButtonMashActor` OtherActor)
  (set `self.CurrentButtonMash` null))

(event `self.ReceiveTick`
  (params (DeltaSeconds :type "Float (single-precision)"))
  (bind _currentbuttonmash (`self.CurrentButtonMash`))
  (bind _playercharacter (`self.PlayerCharacter`))
  (bind _charactermovement (`Character.CharacterMovement` _playercharacter))
  (if (`KismetSystemLibrary.IsValid` _currentbuttonmash)
    (if (`/Game/Blueprints/Weapons/ButtonMashActor.Picking` _currentbuttonmash)
      (bind _asbp_player_controller (cast `/Game/Blueprints/Player/BP_PlayerController` (`self.PlayerController`)))
      (`PlayerController.SetViewTargetWithBlend` _asbp_player_controller (`ChildActorComponent.ChildActor` (`/Game/Blueprints/Player/BP_ThirdPersonCharacter.PickingCamera` _playercharacter)) 0.25 "VTBlend_EaseIn" 1.0 false)
      (`PlayerController.SetViewTargetWithBlend` (`self.PlayerController`) (`ChildActorComponent.ChildActor` (`/Game/Blueprints/Player/BP_ThirdPersonCharacter.PickingCamera` _playercharacter)) 0.25 "VTBlend_EaseIn" 1.0 false)
      (`CharacterMovementComponent.DisableMovement` _charactermovement)
      (else
        (bind _asbp_player_controller_2 (cast `/Game/Blueprints/Player/BP_PlayerController` (`self.PlayerController`) :!label _label))
        (`PlayerController.SetViewTargetWithBlend` _asbp_player_controller_2 (`self.PlayerCharacter`) 0.25 "VTBlend_EaseOut" 1.0 false)
        (`PlayerController.SetViewTargetWithBlend` (`self.PlayerController`) (`self.PlayerCharacter`) 0.25 "VTBlend_EaseOut" 1.0 false)
        (`CharacterMovementComponent.SetMovementMode` _charactermovement (`self.MovementMode`) 0)))
    (else
      (goto _label))))